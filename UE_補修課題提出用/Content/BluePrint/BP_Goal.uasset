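; BP_Goal is the level goal actor that ends a run when its Goal component registers a hit.
; On hit it creates a fresh BP_SaveGame, stores a score computed as 50 minus the BP_GameInstance Timer, and overwrites the SaveGame slot without loading or comparing previous data.
; It then sets BGoal on the game instance and opens the Title level.
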(event `self.Goal.OnComponentHit`
  (params (HitComponent :type "PrimitiveComponent Object Reference") (OtherActor :type "Actor Object Reference") (OtherComp :type "PrimitiveComponent Object Reference") (NormalImpulse :type "Vector Structure") (Hit :type "HitResult Structure (by ref)"))
  (bind _returnvalue (`GameplayStatics.CreateSaveGameObject` "/Game/BluePrint/BP_SaveGame.BP_SaveGame_C"))
  (set `/Game/BluePrint/BP_SaveGame.Save_Score` (- 50 (`/Game/BluePrint/BP_GameInstance.Timer` (cast `/Game/BluePrint/BP_GameInstance` (`GameplayStatics.GetGameInstance`) :!pure true))) _returnvalue)
  (`GameplayStatics.SaveGameToSlot` _returnvalue "SaveGame")
  (set `/Game/BluePrint/BP_GameInstance.b_Goal` true (cast `/Game/BluePrint/BP_GameInstance` (`GameplayStatics.GetGameInstance`) :!pure true))
  (`GameplayStatics.OpenLevel` "Title"))

(fn `UserConstructionScript`)